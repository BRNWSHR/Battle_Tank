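; Mortar Blueprint with a turret, a barrel, an aiming component and a health bar widget.
; On BeginPlay it passes the turret and barrel to the MortarAiming component, then links the widget to this mortar by setting MortarRef on its UI_HealthBar.
; The graphs contain only this setup wiring, with no aiming, firing or damage logic, and the construction script is empty.
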(event `self.ReceiveBeginPlay`
  (`TankAimingComponent.Initialise` (`self.MortarAiming`) (`self.MortarTurret`) (`self.MortarBarrel`))
  (`self.InitialiseHealthBar`))

(fn `InitialiseHealthBar`
  (bind _asui_health_bar (cast `/Game/Blueprints/UI/UI_HealthBar` (`WidgetComponent.GetUserWidgetObject` (`self.Widget`))))
  (set `/Game/Blueprints/UI/UI_HealthBar.MortarRef` self _asui_health_bar))

(fn `UserConstructionScript`)